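; Player state that loads or creates the save, sets up the player character's abilities and manages pause and settings menus.
; BeginPlay reads character status and ability levels from the save slot, then grants Move, AirStop and NbleJump GAS abilities at those levels and creates both menu widgets.
; ActivateUI keeps a stack of opened widgets, restoring the previous one on close and toggling the cursor.
; SaveCurrentStatus and UpdateCharacterAbilityLevel are empty stubs.
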(event EventBeginPlay
  (bind _slot_name (Variables|Default|GetSlot%20Name))
  ;[1 1 1 1 50] Load
  (bind _returnvalue (SaveGame|DoesSaveGameExist _slot_name))
  (if _returnvalue
    (bind _returnvalue_2 (SaveGame|LoadGamefromSlot _slot_name))
    (bind _asbp_save_data (Utilities|Casting|CastToBP_SaveData _returnvalue_2))
    (Variables|Default|SetST%20Player%20Character (.characterstatus (Variables|/Game/Blueprints/BP_SaveData.BP_SaveData_C|GetSaveData _asbp_save_data)))
    (bind _output_get (Variables|Default|SetST%20Player%20Ability%20Level (.abilitystatus (Variables|/Game/Blueprints/BP_SaveData.BP_SaveData_C|GetSaveData _asbp_save_data))))
    (else
      (CallFunction|SaveCurrentStatus)
      (bind _returnvalue_3 (SaveGame|CreateSaveGameObject "/Game/Blueprints/BP_SaveData.BP_SaveData_C"))
      (Variables|/Game/Blueprints/BP_SaveData.BP_SaveData_C|SetSaveData _returnvalue_3 (Utilities|Struct|MakeST_PlayerStatus (Variables|Default|GetST%20Player%20Character) (Variables|Default|GetST%20Player%20Ability%20Level)))
      (SaveGame|SaveGametoSlot _returnvalue_3 _slot_name)))
  (bind _asbp_third_person_character (Utilities|Casting|CastToBP_ThirdPersonCharacter (Game|GetPlayerCharacter 0)))
  (bind _output_get_2 (Variables|Default|SetCharacterComponent _asbp_third_person_character))
  (Default|UpdateAbilityStatus _asbp_third_person_character _output_get)
  (bind _returnvalue_4 (AddComponent|AddAbilitySystemComponent _output_get_2))
  ;[1 1 1 1 50] Ability
  (bind _output_get_3 (Variables|/Script/JEXPR.JEXPRCharacter|SetAbilitySystemComponent _output_get_2 _returnvalue_4))
  (bind _returnvalue_5 (GameplayAbilities|GiveAbility _output_get_3 "/Game/Blueprints/Abilities/GA_Move.GA_Move_C" (.levelcharge (Variables|Default|GetST%20Player%20Ability%20Level)) -1))
  (bind _returnvalue_6 (GameplayAbilities|GiveAbility _output_get_3 "/Game/Blueprints/Abilities/GA_AirStop.GA_AirStop_C" (.levelairstop (Variables|Default|GetST%20Player%20Ability%20Level)) -1))
  (bind _returnvalue_7 (GameplayAbilities|GiveAbility _output_get_3 "/Game/Blueprints/Abilities/GA_NbleJump.GA_NbleJump_C" (.leveljump (Variables|Default|GetST%20Player%20Ability%20Level)) -1))
  (bind _output_get_4 (Variables|Default|SetST%20Player%20Ability%20Spec (Utilities|Struct|MakeST_AbilitySpecs _returnvalue_6 _returnvalue_5 _returnvalue_7)))
  (Default|InitAbilityandSpec (Variables|Default|GetCharacterComponent) _output_get_3 _output_get_4)
  ;[1 1 1 1 50] Widget
  (bind _returnvalue_8 (UserInterface|CreateWidget "/Game/Blueprints/UI/WB_PauseSettingUI.WB_PauseSettingUI_C" (Game|GetPlayerController 0)))
  (Variables|Default|SetWB_PauseSettingWidget _returnvalue_8)
  (bind _returnvalue_9 (UserInterface|CreateWidget "/Game/Blueprints/UI/WB_SettingUI.WB_SettingUI_C"))
  (Variables|Default|SetWB_SettingWidget _returnvalue_9))

(fn ConstructionScript)

(fn SaveCurrentStatus)

(fn UpdateCharacterAbilityLevel
  (params (AbilityStatus :type ST%20Ability%20Status%20Structure)))

(fn ActivateUI
  (params (UI%20Enum :type Enum_UI%20Enum :default "NewEnumerator0") (Activate :type Boolean))
  (bind _wb_settingwidget (Variables|Default|GetWB_SettingWidget))
  (bind _openedwidgetlist (Variables|Default|GetOpenedWidgetList))
  (bind _wb_pausesettingwidget (Variables|Default|GetWB_PauseSettingWidget))
  (bind _openedwidgetlist_2 (Variables|Default|GetOpenedWidgetList))
  (bind _returnvalue (Utilities|Array|LastIndex _openedwidgetlist_2))
  (Viewport|RemoveAllWidgets)
  (if Activate
    (Variables|/Script/Engine.PlayerController|SetbShowMouseCursor (Game|GetPlayerController) true)
    (switch Utilities|FlowControl|Switch|SwitchonEnum_UI UI%20Enum
      (:NewEnumerator0
        (UserInterface|Viewport|AddtoPlayerScreen _wb_pausesettingwidget)
        (Utilities|Array|Add _openedwidgetlist _wb_pausesettingwidget))
      (:NewEnumerator1
        (UserInterface|Viewport|AddtoPlayerScreen _wb_settingwidget)
        (Utilities|Array|Add _openedwidgetlist _wb_settingwidget)))
    (return false)
    (else
      (Utilities|Array|RemoveIndex _openedwidgetlist_2 _returnvalue)
      (if (Utilities|Array|IsEmpty _openedwidgetlist_2)
        (Variables|/Script/Engine.PlayerController|SetbShowMouseCursor (Game|GetPlayerController) false)
        (return true)
        (else
          (bind _returnvalue_2 (UserInterface|Viewport|AddtoPlayerScreen (Utilities|Array|Get(acopy) _openedwidgetlist_2 _returnvalue)))
          (return (not _returnvalue_2)))))))