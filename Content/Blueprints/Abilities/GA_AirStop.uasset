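; GA_AirStop is a gameplay ability that freezes the player character in midair.
; Activation commits, zeroes gravity scale and velocity, then ends on input release or after a one-second delay, restoring a hard-coded gravity scale on end.
; It can activate only while off the ground and when the character's CanAirStop check passes; each commit calls DiscountAirStopCount on the character.
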(event Ability|EventActivateAbility
  (bind _asbp_third_person_character (Utilities|Casting|CastToBP_ThirdPersonCharacter (Game|GetPlayerCharacter 0)))
  (Ability|CommitAbility)
  (Variables|/Script/Engine.CharacterMovementComponent|SetGravityScale (Variables|/Script/Engine.Character|GetCharacterMovement _asbp_third_person_character) 0.0)
  (Variables|/Script/Engine.MovementComponent|SetVelocity (Variables|/Script/Engine.Character|GetCharacterMovement _asbp_third_person_character) "0, 0, 0")
  (Ability|Tasks|WaitInputRelease false
    (:then
      (Ability|Tasks|WaitDelay 1.0
        (:OnFinish
          (Ability|EndAbility))))
    (:OnRelease
      (Ability|EndAbility))))

(event Ability|EventOnEndAbility
  (params (bWasCancelled :type Boolean))
  (Variables|/Script/Engine.CharacterMovementComponent|SetGravityScale (Variables|/Script/Engine.Character|GetCharacterMovement (stale Ability|EventActivateAbility _asbp_third_person_character)) 1.75))

(event Ability|EventCommitExecute
  (Class|JEXPRCharacter|DiscountAirStopCount (stale Ability|EventActivateAbility _asbp_third_person_character)))

(fn K2CanActivateAbility
  (params (ActorInfo :type Gameplay%20Ability%20Actor%20Info%20Structure) (Handle :type Gameplay%20Ability%20Spec%20Handle%20Structure))
  (bind _asbp_third_person_character (Utilities|Casting|CastToBP_ThirdPersonCharacter (.owneractor ActorInfo)))
  (bind _asbp_third_person_character_2 (Utilities|Casting|CastToBP_ThirdPersonCharacter (Game|GetPlayerCharacter 0)))
  (return "(GameplayTags=((TagName=\"AirStop\")))" (and (Class|JEXPRCharacter|CanAirStop _asbp_third_person_character) (not (AI|Components|NavMovement|IsMovingonGround (Variables|/Script/Engine.Character|GetCharacterMovement _asbp_third_person_character_2))))))