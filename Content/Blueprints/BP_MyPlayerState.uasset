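; Player state Blueprint that holds the player's character and ability status and initializes both from a save slot on BeginPlay.
; If a save exists, it copies the BP_SaveData contents into its variables without applying them to the pawn.
; Otherwise, SaveCurrentStatus records the pawn's transform in both character status fields, and a new save is written with that and the current ability status.
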(event EventBeginPlay
  (bind _slot_name (Variables|Default|GetSlot%20Name))
  (bind _returnvalue (SaveGame|DoesSaveGameExist _slot_name))
  (if _returnvalue
    (bind _returnvalue_2 (SaveGame|LoadGamefromSlot _slot_name))
    (bind _asbp_save_data (Utilities|Casting|CastToBP_SaveData _returnvalue_2))
    (Variables|Default|SetPlayer%20Character (.characterstatus (Variables|/Game/Blueprints/BP_SaveData.BP_SaveData_C|GetSaveData _asbp_save_data)))
    (Variables|Default|SetPlayer%20Ability (.abilitystatus (Variables|/Game/Blueprints/BP_SaveData.BP_SaveData_C|GetSaveData _asbp_save_data)))
    (else
      (CallFunction|SaveCurrentStatus)
      (bind _returnvalue_3 (SaveGame|CreateSaveGameObject "/Game/Blueprints/BP_SaveData.BP_SaveData_C"))
      (Variables|/Game/Blueprints/BP_SaveData.BP_SaveData_C|SetSaveData _returnvalue_3 (Utilities|Struct|MakeStruct_PlayerStatus (Variables|Default|GetPlayer%20Character) (Variables|Default|GetPlayer%20Ability)))
      (SaveGame|SaveGametoSlot _returnvalue_3 _slot_name))))

(fn ConstructionScript)

(fn SaveCurrentStatus
  (bind _returnvalue (Game|Player|GetPlayerPawn 0))
  (bind _returnvalue_2 (Transformation|GetActorTransform _returnvalue))
  (Variables|Default|SetPlayer%20Character (Utilities|Struct|MakeCharacterStatus _returnvalue_2 _returnvalue_2)))